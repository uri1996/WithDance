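; Test Blueprint for talking to three serial COM port devices at once, printing their replies on screen.
; BeginPlay opens the ports through InitSerial and starts a fast looping timer that polls one port per tick, round-robin via a modulo counter.
; Each poll sends "SEND", reads a line, reports it or an error through PrintSerial, then flushes.
; EndPlay closes all three ports.
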(event `self.ReceiveBeginPlay`
  (bind (_serialtarget _portopened) (`self.InitSerial` 15 115200))
  (set `self.SerialPort0` _serialtarget)
  (set `self.Port Opened0` _portopened)
  (bind (_serialtarget_2 _portopened_2) (`self.InitSerial` 13 115200))
  (set `self.SerialPort1` _serialtarget_2)
  (set `self.Port Opened1` _portopened_2)
  (bind (_serialtarget_3 _portopened_3) (`self.InitSerial` 14 115200))
  (set `self.SerialPort2` _serialtarget_3)
  (set `self.Port Opened2` _portopened_3)
  (set `self.i` 0)
  (`KismetSystemLibrary.K2_SetTimerDelegate` (delegate `CustomEvent`) 0.05 true true))

(event `CustomEvent`
  (bind _serialport0 (`self.SerialPort0`))
  (bind _serialport1 (`self.SerialPort1`))
  (bind _serialport2 (`self.SerialPort2`))
  (switch `int` (mod (`self.i`) 3)
    (:`0`
      (`SerialCom.Println` _serialport0 "SEND")
      (bind (_bsuccess _returnvalue) (`SerialCom.Readln` _serialport0))
      (`self.PrintSerial` (`self.Port Opened0`) _bsuccess 15 _returnvalue)
      (`SerialCom.Flush` (`self.SerialPort0`)))
    (:`1`
      (`SerialCom.Println` _serialport1 "SEND")
      (bind (_bsuccess_2 _returnvalue_2) (`SerialCom.Readln` _serialport1))
      (`self.PrintSerial` (`self.Port Opened1`) _bsuccess_2 13 _returnvalue_2)
      (`SerialCom.Flush` (`self.SerialPort1`)))
    (:`2`
      (`SerialCom.Println` _serialport2 "SEND")
      (bind (_bsuccess_3 _returnvalue_3) (`SerialCom.Readln` _serialport2))
      (`self.PrintSerial` (`self.Port Opened2`) _bsuccess_3 14 _returnvalue_3)
      (`SerialCom.Flush` (`self.SerialPort2`))))
  (set `self.i` (+ (`self.i`) 1)))

(event `self.ReceiveEndPlay`
  (params (EndPlayReason :type "EEndPlayReason Enum" :default "Destroyed"))
  (`SerialCom.Close` (`self.SerialPort0`))
  (`SerialCom.Close` (`self.SerialPort1`))
  (`SerialCom.Close` (`self.SerialPort2`)))

(fn `InitSerial`
  (params (NumPort :type Integer) (NumBaud :type Integer))
  (returns (SerialTarget :type "SerialCom Object Reference") (PortOpened :type Boolean))
  (bind (_bopened _returnvalue) (`SerialCom.OpenComPort` NumPort NumBaud))
  (if _bopened
    (`SerialCom.Flush` _returnvalue)
    (return _returnvalue _bopened)
    (else
      (`KismetSystemLibrary.PrintString` "PORT IS NOT CONNECTED!!!"))))

(fn `PrintSerial`
  (params (isOpened :type Boolean) (isSucceed :type Boolean) (NumPort :type Integer) (SerialString :type String))
  (bind _returnvalue (`KismetStringLibrary.Concat_StrStr` "COM" (`KismetStringLibrary.Conv_IntToString` NumPort) ": "))
  (if isOpened
    (if isSucceed
      (`KismetSystemLibrary.PrintString` (`KismetStringLibrary.Concat_StrStr` _returnvalue SerialString))
      (else
        (`KismetSystemLibrary.PrintString` (`KismetStringLibrary.Concat_StrStr` _returnvalue "Failed to Read!"))))
    (else
      (`KismetSystemLibrary.PrintString` (`KismetStringLibrary.Concat_StrStr` "" "Not Opened!")))))

(fn `UserConstructionScript`)