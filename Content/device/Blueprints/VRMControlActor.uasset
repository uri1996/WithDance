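; Test actor that drives a VRM avatar's hip, thigh and knee bones from three serial-port trackers for waist and legs.
; It opens the COM ports on BeginPlay and closes them on EndPlay, with keys to reopen, close or send RESET.
; Tick polls one tracker per frame in rotation to avoid collisions, sending SEND and parsing the comma-separated reply into two rotators applied in component space.
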(event `Key|LeftBracket`
  (params (Key :type "Key Structure"))
  (:`Pressed`
    (bind (_isopened _serialtarget) (`self.InitSerial` 5 115200 :!label _label)) ; 腰用トラッカーの初期化
    (set `self.SerialPort0` _serialtarget)
    (bind (_isopened_2 _serialtarget_2) (`self.InitSerial` 10 115200)) ; 左脚用トラッカーの初期化
    (set `self.SerialPort1` _serialtarget_2)
    (bind (_isopened_3 _serialtarget_3) (`self.InitSerial` 9 115200)) ; 右脚用トラッカーの初期化
    (set `self.SerialPort2` _serialtarget_3)
    (set `self.i` 0) ; ループカウンタ
  ))

(event `self.ReceiveBeginPlay`
  (goto _label))

(event `Key|@`
  (params (Key :type "Key Structure"))
  (:`Pressed`
    (`SerialCom.Close` (`self.SerialPort0`) :!label _label_2) ; 終了時にシリアルポートを閉じる。これがないと、再接続に影響が出ると思われる
    (`SerialCom.Close` (`self.SerialPort1`))
    (`SerialCom.Close` (`self.SerialPort2`))))

(event `self.ReceiveEndPlay`
  (params (EndPlayReason :type "EEndPlayReason Enum" :default "Destroyed"))
  (goto _label_2))

(event `self.ReceiveTick`
  (params (DeltaSeconds :type "Float (single-precision)"))
  (bind _vrmposeablemesh (`self.VrmPoseableMesh`))
  (bind _vrmposeablemesh_2 (`self.VrmPoseableMesh`))
  (bind _returnvalue (`PoseableMeshComponent.GetBoneRotationByName` (`self.VrmPoseableMesh`) "10_joint_HipMaster" "WorldSpace"))
  (`KismetSystemLibrary.PrintString` (`KismetStringLibrary.Conv_RotatorToString` _returnvalue))
  (switch `int` (mod (`self.i`) 3)
    (:`0`
      (bind (_issucceeed _angle1) (`self.ReadTracker` (`self.SerialPort0`))) ; 値を読みだす関数
      (if _issucceeed
        (`PoseableMeshComponent.SetBoneRotationByName` (`self.VrmPoseableMesh`) "10_joint_HipMaster" _angle1 "ComponentSpace") ; Hip(腰)ボーンを動かす(動作確認用)
      ))
    (:`1`
      (bind (_issucceeed_2 _angle1_2 _angle2) (`self.ReadTracker` (`self.SerialPort1`))) ; 値を読みだす関数
      (if _issucceeed_2
        (`PoseableMeshComponent.SetBoneRotationByName` _vrmposeablemesh_2 "95_joint_LeftHip" _angle1_2 "ComponentSpace") ; LeftHip(左太もも)ボーンを動かす(動作確認用)
        (`PoseableMeshComponent.SetBoneRotationByName` _vrmposeablemesh_2 "96_joint_LeftKnee" _angle2 "ComponentSpace") ; LeftKnee(左ひざ下)ボーンを動かす(動作確認用)
      ))
    (:`2`
      (bind (_issucceeed_3 _angle1_3 _angle2_2) (`self.ReadTracker` (`self.SerialPort2`))) ; 値を読みだす関数
      (if _issucceeed_3
        (`PoseableMeshComponent.SetBoneRotationByName` _vrmposeablemesh "89_joint_RightHip" _angle1_3 "ComponentSpace") ; RightHip(右太もも)ボーンを動かす(動作確認用)
        (`PoseableMeshComponent.SetBoneRotationByName` _vrmposeablemesh "90_joint_RightKnee" _angle2_2 "ComponentSpace") ; RightKnee(右ひざ下)ボーンを動かす(動作確認用)
      )))
  (set `self.i` (+ (`self.i`) 1)) ; iを更新
)

(event `Key|R`
  (params (Key :type "Key Structure"))
  (:`Pressed`
    (`SerialCom.Println` (`self.SerialPort0`) "RESET") ; リセットする(マイコン内に、文字列RESETを受信したらリセットするプログラムを用意してある)
    (`SerialCom.Println` (`self.SerialPort1`) "RESET")
    (`SerialCom.Println` (`self.SerialPort2`) "RESET")))

(fn `ConvertStringToRotator`
  (params (InputString :type String))
  (returns (Rotator1 :type "Rotator Structure") (Rotator2 :type "Rotator Structure"))
  (for (_array_element _array_index) (`KismetStringLibrary.ParseIntoArray` InputString ",")
    (switch `int` _array_index ; 要素番号をもとに、各要素ごとに分岐
      (:`0`
        (bind _returnvalue (`KismetStringLibrary.Conv_StringToDouble` _array_element))
        (bind _output_get (set `self.Pitch` _returnvalue)))
      (:`1`
        (bind _output_get_2 (set `self.Roll` _returnvalue)))
      (:`2`
        (bind _output_get_3 (set `self.Yaw` _returnvalue)))
      (:`3`
        (bind _output_get_4 (set `self.Pitch2` _returnvalue)))
      (:`4`
        (bind _output_get_5 (set `self.Roll2` _returnvalue)))
      (:`5`
        (set `self.Yaw2` _returnvalue))))
  (return (`KismetMathLibrary.MakeRotator` _output_get_2 _output_get _output_get_3) (`KismetMathLibrary.MakeRotator` _output_get_5 _output_get_4)) ; 2つのRotatorを出力
)

(fn `InitSerial`
  (params (NumPort :type Integer) (NumBaud :type Integer))
  (returns (isOpened :type Boolean) (SerialTarget :type "SerialCom Object Reference"))
  (bind (_bopened _returnvalue) (`SerialCom.OpenComPort` NumPort NumBaud)) ; まずポートを開く
  (if _bopened
    (`SerialCom.Flush` _returnvalue) ; 一度ポート内のデータをすべて消費してきれいにする(っていう感じか？)
    (else
      (`KismetSystemLibrary.PrintString` "PORT IS NOT CONNECTED!!!")))
  (return _bopened _returnvalue) ; ポートが開いたかの情報と、開いた\nシリアルポートのターゲットオブジェクトを返す
)

(fn `ReadTracker`
  (params (SerialTarget :type "SerialCom Object Reference"))
  (returns (isSucceeed :type Boolean) (Angle1 :type "Rotator Structure") (Angle2 :type "Rotator Structure"))
  (`SerialCom.Println` SerialTarget "SEND") ; まず、読みたいトラッカーに向けて\n文字列SENDを送信(データの衝突防止)
  (bind (_bsuccess _returnvalue) (`SerialCom.Readln` SerialTarget)) ; 送られてきたデータを1行読む
  (if _bsuccess
    (bind (_rotator1 _rotator2) (`self.ConvertStringToRotator` _returnvalue)) ; 送られた文字列を2組の角度データに変える。\n意外と大掛かりな処理なので関数化している
    (`SerialCom.Flush` SerialTarget) ; バグ防止でいったんデータを掃除
  )
  (return _bsuccess _rotator1 _rotator2) ; 読めたかどうかと、2組の角度情報を返す
)

(fn `UserConstructionScript`)