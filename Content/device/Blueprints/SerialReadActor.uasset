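; Actor that reads text from a serial COM port, likely for an external device, and prints it on screen.
; BeginPlay opens a hard-coded port with flow control, stores and flushes it if open, and prints the connection status.
; Tick polls the port with ReadString every frame, storing successful reads in StrSerial and printing them, and EndPlay closes the port.
; Line-based reading and a RESET write are left unwired.
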(event `self.ReceiveBeginPlay`
  (bind (_bopened _returnvalue) (`SerialCom.OpenComPortWithFlowControl` 15 115200))
  (if (`SerialCom.IsOpened` _returnvalue)
    (bind _output_get (set `self.MySerialPort` _returnvalue))
    (`SerialCom.Flush` _output_get)
    (`KismetSystemLibrary.PrintString` "PORT IS INITIALIZED!!!")
    (else
      (`KismetSystemLibrary.PrintString` "PORT IS NOT CONNECTED!!!"))))

(event `self.ReceiveEndPlay`
  (params (EndPlayReason :type "EEndPlayReason Enum" :default "Destroyed"))
  (`SerialCom.Close` (`self.MySerialPort`)))

(event `self.ReceiveTick`
  (params (DeltaSeconds :type "Float (single-precision)"))
  (bind (_bsuccess _returnvalue) (`SerialCom.ReadString` (`self.MySerialPort`)))
  (if _bsuccess
    (bind _output_get (set `self.StrSerial` _returnvalue))
    (`KismetSystemLibrary.PrintString` _output_get)))

(fn `UserConstructionScript`)