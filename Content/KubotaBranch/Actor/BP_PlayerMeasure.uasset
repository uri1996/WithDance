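; BP_PlayerMeasure calibrates the VR player's body, saving head height and hand positions for arms out, arms up and a third pose to VR_Debug_GameMode.
; BP_tutorialEvent callbacks or H/V keys trigger arm measurements; M and D keys capture head height and the third pose.
; H/V captures require both hands to be still since the previous check, read controller positions after a delay, then fire one-time success dispatchers.
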(event `self.ReceiveBeginPlay`
  (bind _asvr_debug_pawn (cast `/Game/KubotaBranch/Debug/VR_Debug_Pawn` (`GameplayStatics.GetPlayerPawn` 0)))
  (set `self.PlayerPawn` _asvr_debug_pawn)
  (bind _asvr_debug_game_mode (cast `/Game/KubotaBranch/Debug/VR_Debug_GameMode` (`GameplayStatics.GetGameMode`)))
  (set `self.GameMode` _asvr_debug_game_mode)
  (bind _outactors (`GameplayStatics.GetAllActorsOfClass` "/Game/KubotaBranch/tutorial/BP_tutorialEvent.BP_tutorialEvent_C"))
  (bind _output (`|GetArrayItem` _outactors))
  (add `/Game/KubotaBranch/tutorial/BP_tutorialEvent.CallMeasureHandH` _output (delegate `MeasureH`))
  (add `/Game/KubotaBranch/tutorial/BP_tutorialEvent.CallMeasureHandV` _output (delegate `MeasureV`)))

(event `Key|H`
  (params (Key :type "Key Structure"))
  (bind _playerpawn (`self.PlayerPawn`))
  (bind _gamemode (`self.GameMode`))
  (bind (_returnvalue_x _returnvalue_y) (`KismetMathLibrary.BreakVector` (`SceneComponent.K2_GetComponentLocation` (`/Game/KubotaBranch/Debug/VR_Debug_Pawn.MotionControllerLeftGrip` _playerpawn))))
  (bind (_returnvalue_x_2 _returnvalue_y_2) (`KismetMathLibrary.BreakVector` (`SceneComponent.K2_GetComponentLocation` (`/Game/KubotaBranch/Debug/VR_Debug_Pawn.MotionControllerRightGrip` _playerpawn))))
  ;[1 1 1] 手を横に広げた時の最大値の取得
  (:`Pressed`
    (`KismetSystemLibrary.Delay` 1.0 :!label _label)
    (set `self.FreezeFlag` false)
    (bind _value (`self.IsPlayerFreeze`))
    (if (and _value (`self.FinishH`))
      (`KismetSystemLibrary.PrintString` "3秒後読み取り")
      (`KismetSystemLibrary.Delay` 3.0)
      (bind _output_get (set `/Game/KubotaBranch/Debug/VR_Debug_GameMode.LArmLength_H` _returnvalue_y _gamemode))
      (`KismetSystemLibrary.PrintString` (`KismetStringLibrary.Conv_DoubleToString` _output_get))
      (bind _output_get_2 (set `/Game/KubotaBranch/Debug/VR_Debug_GameMode.RArmLength_H` _returnvalue_y_2 _gamemode))
      (`KismetSystemLibrary.PrintString` (`KismetStringLibrary.Conv_DoubleToString` _output_get_2))
      (set `self.FinishH` false)
      (`self.CallMeasureHSuccess`))))

(event `MeasureH`
  ;[1 1 1] 手を横に広げた時の最大値の取得
  (goto _label))

(event `Key|M`
  (params (Key :type "Key Structure"))
  (bind (_returnvalue_x _returnvalue_y _returnvalue_z) (`KismetMathLibrary.BreakVector` (`SceneComponent.K2_GetComponentLocation` (`/Game/KubotaBranch/Debug/VR_Debug_Pawn.HeadMountedDisplayMesh` (`self.PlayerPawn`)))))
  (:`Pressed`
    (bind _output_get (set `/Game/KubotaBranch/Debug/VR_Debug_GameMode.HeadHight` _returnvalue_z (`self.GameMode`)))
    (`KismetSystemLibrary.PrintString` (`KismetStringLibrary.Conv_DoubleToString` _output_get))))

(event `Key|V`
  (params (Key :type "Key Structure"))
  (bind _gamemode (`self.GameMode`))
  (bind _playerpawn (`self.PlayerPawn`))
  (bind (_returnvalue_x _returnvalue_y _returnvalue_z) (`KismetMathLibrary.BreakVector` (`SceneComponent.K2_GetComponentLocation` (`/Game/KubotaBranch/Debug/VR_Debug_Pawn.MotionControllerLeftGrip` _playerpawn))))
  (bind (_returnvalue_x_2 _returnvalue_y_2 _returnvalue_z_2) (`KismetMathLibrary.BreakVector` (`SceneComponent.K2_GetComponentLocation` (`/Game/KubotaBranch/Debug/VR_Debug_Pawn.MotionControllerRightGrip` _playerpawn))))
  ;[1 1 1] 手を上に上げた時の最大値の取得
  (:`Pressed`
    (`KismetSystemLibrary.Delay` 1.0 :!label _label_2)
    (set `self.FreezeFlag` false)
    (bind _value (`self.IsPlayerFreeze`))
    (if (and _value (`self.FinishV`))
      (`KismetSystemLibrary.PrintString` "3秒後読み取り")
      (`KismetSystemLibrary.Delay` 3.0)
      (bind _output_get (set `/Game/KubotaBranch/Debug/VR_Debug_GameMode.LArmLength_V` _returnvalue_z _gamemode))
      (`KismetSystemLibrary.PrintString` (`KismetStringLibrary.Conv_DoubleToString` _output_get))
      (bind _output_get_2 (set `/Game/KubotaBranch/Debug/VR_Debug_GameMode.RArmLength_V` _returnvalue_z_2 _gamemode))
      (`KismetSystemLibrary.PrintString` (`KismetStringLibrary.Conv_DoubleToString` _output_get_2))
      (set `self.FinishV` false)
      (`self.CallMesureVSuccess`))))

(event `MeasureV`
  ;[1 1 1] 手を上に上げた時の最大値の取得
  (goto _label_2))

(event `Key|D`
  (params (Key :type "Key Structure"))
  (bind _playerpawn (`self.PlayerPawn`))
  (bind _gamemode (`self.GameMode`))
  (bind (_returnvalue_x _returnvalue_y _returnvalue_z) (`KismetMathLibrary.BreakVector` (`SceneComponent.K2_GetComponentLocation` (`/Game/KubotaBranch/Debug/VR_Debug_Pawn.MotionControllerLeftGrip` _playerpawn))))
  (bind (_returnvalue_x_2 _returnvalue_y_2 _returnvalue_z_2) (`KismetMathLibrary.BreakVector` (`SceneComponent.K2_GetComponentLocation` (`/Game/KubotaBranch/Debug/VR_Debug_Pawn.MotionControllerRightGrip` _playerpawn))))
  (:`Pressed`
    (`KismetSystemLibrary.PrintString` "3秒後読み取り")
    (`KismetSystemLibrary.Delay` 3.0)
    (bind _output_get (set `/Game/KubotaBranch/Debug/VR_Debug_GameMode.LArmLength_D` _returnvalue_z _gamemode))
    (`KismetSystemLibrary.PrintString` (`KismetStringLibrary.Conv_DoubleToString` _output_get))
    (bind _output_get_2 (set `/Game/KubotaBranch/Debug/VR_Debug_GameMode.RArmLength_D` _returnvalue_z_2 _gamemode))
    (`KismetSystemLibrary.PrintString` (`KismetStringLibrary.Conv_DoubleToString` _output_get_2))))

(fn `IsPlayerFreeze`
  (returns (value :type Boolean))
  (bind _playerpawn (`self.PlayerPawn`))
  (bind _returnvalue (`SceneComponent.K2_GetComponentLocation` (`/Game/KubotaBranch/Debug/VR_Debug_Pawn.MotionControllerLeftGrip` _playerpawn)))
  (bind _returnvalue_2 (`SceneComponent.K2_GetComponentLocation` (`/Game/KubotaBranch/Debug/VR_Debug_Pawn.MotionControllerRightGrip` _playerpawn)))
  (bind _output_get (set `self.FreezeFlag` (and (<= (`KismetMathLibrary.VSize` (- _returnvalue (`self.AfterHandL`))) 1.0) (<= (`KismetMathLibrary.VSize` (- _returnvalue_2 (`self.AfterHandR`))) 1.0))))
  (set `self.AfterHandL` _returnvalue)
  (set `self.AfterHandR` _returnvalue_2)
  (`KismetSystemLibrary.PrintString` (`KismetStringLibrary.Conv_BoolToString` _output_get))
  (return _output_get))

(fn `UserConstructionScript`)