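; Music clock actor for the VR dance mode that times note spawning to the song and ends playback at the last timing entry.
; StartAudio, also bound to the O key, creates a Quartz clock, queues the track quantized, then subscribes to bar events.
; Each bar found in the GameInstance's TimingData makes GenerateNote spawn hand and foot notes from AdjustDanceData.
; StopClock and RestartClock pause and resume sound and clock together.
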(event `RestartClock`
  (`AudioComponent.SetPaused` (`self.Sound`) false)
  (bind _clockhandle (`QuartzClockHandle.StartClock` (`self.NewClock`)))
  (set `self.NewClock` _clockhandle))

(event `self.ReceiveBeginPlay`
  (bind _outactors (`GameplayStatics.GetAllActorsOfClass` "/Game/KubotaBranch/Actor/GenerateNote.GenerateNote_C"))
  (bind _output_get (set `self.GenerateNote` (`|GetArrayItem` _outactors)))
  (`KismetSystemLibrary.PrintString` (`KismetStringLibrary.Conv_BoolToString` (`KismetSystemLibrary.IsValid` _output_get)))
  (bind _asvr_dance_mode (cast `/Game/KubotaBranch/Debug/VR_DanceMode` (`GameplayStatics.GetGameMode`)))
  (set `self.GameMode` _asvr_dance_mode)
  (bind _outactors_2 (`GameplayStatics.GetAllActorsOfClass` "/Game/KubotaBranch/Motion/BP_DanceChara.BP_DanceChara_C"))
  (set `self.chara` (`|GetArrayItem` _outactors_2))
  (bind _asproject_game_instance (cast `/Game/Main/Blueprints/Project_GameInstance` (`GameplayStatics.GetGameInstance`)))
  (set `self.gameInstance` _asproject_game_instance)
  (`KismetSystemLibrary.PrintString` "出現できてる"))

(event `StopClock`
  (`AudioComponent.SetPaused` (`self.Sound`) true)
  (bind _clockhandle (`QuartzClockHandle.PauseClock` (`self.NewClock`)))
  (set `self.NewClock` _clockhandle))

(event `StartAudio`
  (bind _returnvalue (`QuartzSubsystem.CreateNewClock` (subsystem `QuartzSubsystem`) "NewClock" (make `QuartzClockSettings` (make `QuartzTimeSignature` 4 "SixteenthNote")) false true :!label _label))
  (bind _clockhandle (`QuartzClockHandle.SetBeatsPerMinute` :`self` _returnvalue :`BeatsPerMinute` 145.0))
  (set `self.NewClock` _clockhandle)
  (bind _returnvalue_2 (`GameplayStatics.CreateSound2D` "/Game/KubotaBranch/Music/Say_Say_Do_Do_cutVer2.Say_Say_Do_Do_cutVer2" 1.0 1.0 (`self.Playback Time`) null))
  (bind _output_get (set `self.Sound` _returnvalue_2))
  (add `AudioComponent.OnAudioPlaybackPercent` _output_get (delegate `Playing Sound`))
  (`AudioComponent.PlayQuantized` _output_get (`self.NewClock`) (make `QuartzQuantizationBoundary` "Bar" 1.0 "TransportRelative") (delegate `Cued`) 0.0 0.0 1.0 "Linear"))

(event `Key|O`
  (params (Key :type "Key Structure"))
  (:`Pressed`
    (goto _label)))

(event `Playing Sound`
  (params (PlayingSoundWave :type "SoundWave Object Reference") (PlaybackPercent :type "Float (single-precision)"))
  (bind _output_get (set `self.Playback Time` PlaybackPercent)))

(event `Quantized`
  (params (ClockName :type Name) (QuantizationType :type "EQuartzCommandQuantization Enum" :default "Bar") (NumBars :type Integer) (Beat :type Integer) (BeatFraction :type "Float (single-precision)"))
  (bind _timingdata (`/Game/Main/Blueprints/Project_GameInstance.TimingData` (`self.gameInstance`)))
  (bind _returnvalue (`KismetArrayLibrary.Array_Find` _timingdata NumBars))
  (bind (_hl_position _hr_position _fl_position _fl_rotator _fr_position) (break `/Game/KubotaBranch/Data/DanceData` (`|GetArrayItem` (`/Game/Main/Blueprints/Project_GameInstance.AdjustDanceData` (`self.gameInstance`)) _returnvalue)))
  (bind _x (.x _fl_position))
  (`KismetSystemLibrary.PrintString` (`KismetStringLibrary.Conv_IntToString` NumBars))
  (if (== _returnvalue (`KismetArrayLibrary.Array_LastIndex` _timingdata))
    (`AudioComponent.Stop` (`self.Sound`))
    (`QuartzClockHandle.StopClock` (`self.NewClock`) true)
    (`self.EndMusic`)
    (elif true
      (if (!= _returnvalue -1)
        (if (!= (.x _hl_position) 0.0)
          (`/Game/KubotaBranch/Actor/GenerateNote.GenerateNote_handL` (`self.GenerateNote`) _hl_position (`self.LimitTime`) (`self.EndPos`)))
        (if (!= (.x _hr_position) 0.0)
          (`/Game/KubotaBranch/Actor/GenerateNote.GenerateNote_handR` (`self.GenerateNote`) _hr_position (`self.LimitTime`) (`self.EndPos`)))
        (`KismetSystemLibrary.PrintString` (`KismetStringLibrary.Concat_StrStr` "左足:" (`KismetStringLibrary.Conv_DoubleToString` _x)))
        (if (!= _x 0.0)
          (`KismetSystemLibrary.PrintString` "左足出現")
          (`/Game/KubotaBranch/Actor/GenerateNote.GenerateNote_footL` :`self` (`self.GenerateNote`) :`fotL_Pos` _fl_position :`LimitTime` (`self.LimitTime`) :`EndPos` (`self.EndPos`)))
        (if (!= (.x _fr_position) 0.0)
          (`KismetSystemLibrary.PrintString` "右足出現")
          (`/Game/KubotaBranch/Actor/GenerateNote.GenerateNote_footR` :`self` (`self.GenerateNote`) :`Fot R_Pos` _fr_position :`LimitTime` (`self.LimitTime`) :`EndPos` (`self.EndPos`))))
      (elif (== NumBars 10)
        (`/Game/KubotaBranch/Motion/BP_DanceChara.StopMotion` (`self.chara`))
        (`QuartzClockHandle.StopClock` (`self.NewClock`) true)
        (`AudioComponent.Stop` (`self.Sound`))))))

(event `Cued`
  (params (EventType :type "EQuartzCommandDelegateSubType Enum" :default "CommandOnFailedToQueue") (Name :type Name))
  (switch `EQuartzCommandDelegateSubType` EventType
    (:`CommandOnQueued`
      (bind _clockhandle (`QuartzClockHandle.StartClock` (`self.NewClock`)))
      (`QuartzClockHandle.SubscribeToQuantizationEvent` _clockhandle "Bar" (delegate `Quantized`)))))

(fn `UserConstructionScript`)