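; Tutorial rhythm clock actor that times hand-note spawning to a music track using Quartz.
; StartAudio or the O key creates a 120 BPM clock and plays the beat sound quantized to the bar, starting the clock once it is queued.
; Each bar is looked up in CheckBeat to spawn left, right or both notes through GenerateNote, positioned by GameMode arm lengths, or to end the music.
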(event `self.ReceiveBeginPlay`
  (bind _outactors (`GameplayStatics.GetAllActorsOfClass` "/Game/KubotaBranch/Actor/GenerateNote.GenerateNote_C"))
  (bind _output_get (set `self.GenerateNote` (`|GetArrayItem` _outactors)))
  (`KismetSystemLibrary.PrintString` (`KismetStringLibrary.Conv_BoolToString` (`KismetSystemLibrary.IsValid` _output_get)))
  (bind _asvr_debug_game_mode (cast `/Game/KubotaBranch/Debug/VR_Debug_GameMode` (`GameplayStatics.GetGameMode`)))
  (set `self.GameMode` _asvr_debug_game_mode)
  (bind _outactors_2 (`GameplayStatics.GetAllActorsOfClass` "/Game/KubotaBranch/Actor/BP_CharaTest.BP_CharaTest_C"))
  (set `self.chara` (`|GetArrayItem` _outactors_2)))

(event `StartAudio`
  (bind _returnvalue (`QuartzSubsystem.CreateNewClock` (subsystem `QuartzSubsystem`) "NewClock" (make `QuartzClockSettings` (make `QuartzTimeSignature` 4 "SixteenthNote")) false true :!label _label))
  (bind _clockhandle (`QuartzClockHandle.SetBeatsPerMinute` :`self` _returnvalue :`BeatsPerMinute` 120.0))
  (set `self.NewClock` _clockhandle)
  (bind _returnvalue_2 (`GameplayStatics.CreateSound2D` "/Game/KubotaBranch/Actor/Test_beat.Test_beat" 1.0 1.0 0.0 null))
  (`AudioComponent.PlayQuantized` _returnvalue_2 (`self.NewClock`) (make `QuartzQuantizationBoundary` "Bar" 1.0 "TransportRelative") (delegate `Cued`) 0.0 0.0 1.0 "Linear"))

(event `Key|O`
  (params (Key :type "Key Structure"))
  (:`Pressed`
    (goto _label)))

(event `Quantized`
  (params (ClockName :type Name) (QuantizationType :type "EQuartzCommandQuantization Enum" :default "Bar") (NumBars :type Integer) (Beat :type Integer) (BeatFraction :type "Float (single-precision)"))
  (bind _gamemode (`self.GameMode`))
  (bind _gamemode_2 (`self.GameMode`))
  (bind _rarmlength_h (`/Game/KubotaBranch/Debug/VR_Debug_GameMode.RArmLength_H` _gamemode))
  (`KismetSystemLibrary.PrintString` (`KismetStringLibrary.Conv_IntToString` NumBars))
  (switch `int` (`KismetArrayLibrary.Array_Find` (`self.CheckBeat`) NumBars)
    (:`0`
      (`KismetSystemLibrary.PrintString` "テンポが4")
      (`/Game/KubotaBranch/Actor/GenerateNote.GenerateNote_handL` (`self.GenerateNote`) (`KismetMathLibrary.MakeVector` 300.0 -20.0 (`/Game/KubotaBranch/Debug/VR_Debug_GameMode.LArmLength_V` (`self.GameMode`)))))
    (:`1`
      (`KismetSystemLibrary.PrintString` "テンポが8")
      (`/Game/KubotaBranch/Actor/GenerateNote.GenerateNote_handR` (`self.GenerateNote`) (`KismetMathLibrary.MakeVector` 300.0 20.0 (`/Game/KubotaBranch/Debug/VR_Debug_GameMode.RArmLength_V` (`self.GameMode`)))))
    (:`2`
      (`KismetSystemLibrary.PrintString` "テンポが12")
      (`/Game/KubotaBranch/Actor/GenerateNote.GenerateNote_handL` (`self.GenerateNote`) (`KismetMathLibrary.MakeVector` 300.0 (`/Game/KubotaBranch/Debug/VR_Debug_GameMode.LArmLength_H` _gamemode_2) (- (`/Game/KubotaBranch/Debug/VR_Debug_GameMode.LArmLength_V` _gamemode_2) 30.0)))
      (`KismetSystemLibrary.PrintString` (`KismetStringLibrary.Conv_DoubleToString` _rarmlength_h))
      (`/Game/KubotaBranch/Actor/GenerateNote.GenerateNote_handR` (`self.GenerateNote`) (`KismetMathLibrary.MakeVector` 300.0 _rarmlength_h (- (`/Game/KubotaBranch/Debug/VR_Debug_GameMode.RArmLength_V` _gamemode) 30.0)))
      (`KismetSystemLibrary.PrintString` "成功"))
    (:`3`
      (`self.MusicEnd`)
      (`AudioComponent.Stop` (stale `StartAudio` _returnvalue_2)))))

(event `Cued`
  (params (EventType :type "EQuartzCommandDelegateSubType Enum" :default "CommandOnFailedToQueue") (Name :type Name))
  (switch `EQuartzCommandDelegateSubType` EventType
    (:`CommandOnQueued`
      (bind _clockhandle (`QuartzClockHandle.StartClock` (`self.NewClock`)))
      (`QuartzClockHandle.SubscribeToQuantizationEvent` _clockhandle "Bar" (delegate `Quantized`)))))

(fn `UserConstructionScript`)