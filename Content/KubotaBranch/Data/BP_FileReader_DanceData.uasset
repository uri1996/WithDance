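; Data loader actor that copies dance choreography and timing data from DataTables into the game instance.
; Its ReadFile event casts to Project_GameInstance, then walks every row of the CSV_Data table, appending each found row to ReadDanceData.
; It then does the same with CSV_TimingData, appending only each row's Timing value to TimingData.
; BeginPlay is empty, so loading happens only when ReadFile is called.
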(event `ReadFile`
  (bind _asproject_game_instance (cast `/Game/Main/Blueprints/Project_GameInstance` (`GameplayStatics.GetGameInstance`)))
  (set `self.gameInstance` _asproject_game_instance)
  ;[1 1 1] ダンスデータの読み込み
  (bind _output_get (set `self.DataTable` "/Game/KubotaBranch/Data/CSV_Data.CSV_Data"))
  (bind _outrownames (`DataTableFunctionLibrary.GetDataTableRowNames` _output_get))
  (for _array_element _outrownames
    (bind _returnvalue (`|GetDataTableRow` (`self.DataTable`) _array_element)
      (:`then`
        (bind _returnvalue_2 (`KismetArrayLibrary.Array_Add` (`/Game/Main/Blueprints/Project_GameInstance.ReadDanceData` (`self.gameInstance`)) _returnvalue)))))
  ;[1 1 1] タイミングデータの読み込み
  (bind _output_get_2 (set `self.DataTable_2` "/Game/KubotaBranch/Data/CSV_TimingData.CSV_TimingData"))
  (bind _outrownames_2 (`DataTableFunctionLibrary.GetDataTableRowNames` _output_get_2))
  (for _array_element_2 _outrownames_2
    (bind _returnvalue_3 (`|GetDataTableRow` (`self.DataTable_2`) _array_element_2)
      (:`then`
        (bind _returnvalue_4 (`KismetArrayLibrary.Array_Add` (`/Game/Main/Blueprints/Project_GameInstance.TimingData` (`self.gameInstance`)) (`.Timing_2_2328DEB74B9AD50765AB14B035331602` (break `/Game/KubotaBranch/Data/TimingData` _returnvalue_3))))))))

(event `self.ReceiveBeginPlay`)

(fn `UserConstructionScript`)