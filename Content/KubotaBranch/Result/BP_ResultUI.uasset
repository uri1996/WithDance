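; BP_ResultUI is an actor that hosts the result screen widget and lets VR hand triggers click on it.
; On BeginPlay it disables the widget's shadow, enables player input, adds the trigger Enhanced Input mapping context and caches Project_GameInstance.
; Left and right trigger start and completion events press and release the left mouse button on the matching VR hand pointer stored in the GameInstance.
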(event `self.ReceiveBeginPlay`
  (`PrimitiveComponent.SetCastShadow` (`self.Widget`) false)
  (`self.EnableInput` (`GameplayStatics.GetPlayerController` 0))
  (message `EnhancedInputSubsystemInterface.AddMappingContext` (pcsubsystem `EnhancedInputLocalPlayerSubsystem` (`GameplayStatics.GetPlayerController` 0)) "/Game/WuBranch/Input/Trigger_Map.Trigger_Map" 2 (struct))
  (bind _asproject_game_instance (cast `/Game/Main/Blueprints/Project_GameInstance` (`GameplayStatics.GetGameInstance`)))
  (set `self.gameInstance` _asproject_game_instance))

(event `EnhancedInput|/Game/WuBranch/Input/Action/Trigger_Left`
  (params (ActionValue :type Boolean) (ElapsedSeconds :type "Float (double-precision)") (TriggeredSeconds :type "Float (double-precision)") (InputAction :type "InputAction Object Reference" :default "/Game/WuBranch/Input/Action/Trigger_Left.Trigger_Left"))
  (bind _vrlefthand (`/Game/Main/Blueprints/Project_GameInstance.VRLeftHand` (`self.gameInstance`)))
  (:`Started`
    (`WidgetInteractionComponent.PressPointerKey` _vrlefthand "LeftMouseButton"))
  (:`Completed`
    (`WidgetInteractionComponent.ReleasePointerKey` _vrlefthand "LeftMouseButton")))

(event `EnhancedInput|/Game/WuBranch/Input/Action/Trigger_Right`
  (params (ActionValue :type Boolean) (ElapsedSeconds :type "Float (double-precision)") (TriggeredSeconds :type "Float (double-precision)") (InputAction :type "InputAction Object Reference" :default "/Game/WuBranch/Input/Action/Trigger_Right.Trigger_Right"))
  (bind _vrrighthand (`/Game/Main/Blueprints/Project_GameInstance.VRRightHand` (`self.gameInstance`)))
  (:`Started`
    (`WidgetInteractionComponent.PressPointerKey` _vrrighthand "LeftMouseButton"))
  (:`Completed`
    (`WidgetInteractionComponent.ReleasePointerKey` _vrrighthand "LeftMouseButton")))

(fn `UserConstructionScript`)