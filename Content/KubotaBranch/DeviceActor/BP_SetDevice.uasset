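; BP_SetDevice is a device actor that reads orientation data from two serial devices and prints it for debugging.
; BeginPlay opens COM ports 3 and 4 through InitSerial, which flushes, sends a greeting and reports connection success or failure; EndPlay closes both.
; Tick reads a line from each port, and ConvertStringToRotator splits the comma-separated pitch, roll, yaw values into two rotators, which are only printed.
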(event `self.ReceiveBeginPlay`
  (`self.Init Serial` 0 3 115200)
  (`self.Init Serial` 1 4 115200))

(event `self.ReceiveEndPlay`
  (params (EndPlayReason :type "EEndPlayReason Enum" :default "Destroyed"))
  (`SerialCom.Close` (`self.DeviceCom0`))
  (`SerialCom.Close` (`self.DeviceCom1`)))

(event `self.ReceiveTick`
  (params (DeltaSeconds :type "Float (single-precision)"))
  (bind (_bsuccess _returnvalue) (`SerialCom.Readln` (`self.DeviceCom0`)))
  (if (not (`KismetStringLibrary.EqualEqual_StrStr` _returnvalue))
    (bind _output_get (set `self.line String` _returnvalue))
    (bind (_rotato1 _rotato2) (`self.Convert String to Rotator` _output_get))
    (`KismetSystemLibrary.PrintString` (`KismetStringLibrary.Concat_StrStr` "1:" (`KismetStringLibrary.Conv_RotatorToString` _rotato1) "2:" (`KismetStringLibrary.Conv_RotatorToString` _rotato2))))
  (bind (_bsuccess_2 _returnvalue_2) (`SerialCom.Readln` (`self.DeviceCom1`)))
  (if (not (`KismetStringLibrary.EqualEqual_StrStr` _returnvalue_2))
    (bind _output_get_2 (set `self.line String` _returnvalue_2))
    (bind (_rotato1_2 _rotato2_2) (`self.Convert String to Rotator` _output_get_2))
    (`KismetSystemLibrary.PrintString` (`KismetStringLibrary.Concat_StrStr` "1:" (`KismetStringLibrary.Conv_RotatorToString` _rotato1_2) "2:" (`KismetStringLibrary.Conv_RotatorToString` _rotato2_2)))))

(fn `Convert String to Rotator`
  (params (`Input String` :type String))
  (returns (Rotato1 :type "Rotator Structure") (Rotato2 :type "Rotator Structure"))
  (for (_array_element _array_index) (`KismetStringLibrary.ParseIntoArray` `Input String` ", ")
    (switch `int` _array_index
      (:`0`
        (bind _returnvalue (`KismetStringLibrary.Conv_StringToDouble` _array_element))
        (bind _output_get (set `self.Pitch` _returnvalue)))
      (:`1`
        (bind _output_get_2 (set `self.Roll` _returnvalue)))
      (:`2`
        (bind _output_get_3 (set `self.Yaw` _returnvalue)))
      (:`3`
        (bind _output_get_4 (set `self.Pitch2` _returnvalue)))
      (:`4`
        (bind _output_get_5 (set `self.Roll2` _returnvalue)))
      (:`5`
        (bind _output_get_6 (set `self.Yaw2` _returnvalue)))))
  (return (`KismetMathLibrary.MakeRotator` _output_get_2 _output_get _output_get_3) (`KismetMathLibrary.MakeRotator` _output_get_5 _output_get_4 _output_get_6)))

(fn `Init Serial`
  (params (ID :type Integer) (Port :type Integer) (`Baud Rate` :type Integer))
  (bind (_bopened _returnvalue) (`SerialCom.OpenComPortWithFlowControl` Port `Baud Rate`))
  (if (`SerialCom.IsOpened` _returnvalue)
    (switch `int` ID
      (:`0`
        (set `self.DeviceCom0` _returnvalue))
      (:`1`
        (set `self.DeviceCom1` _returnvalue)))
    (`SerialCom.Flush` _returnvalue)
    (`SerialCom.Println` _returnvalue "we are connected")
    (`KismetSystemLibrary.PrintString` "接続成功")
    (else
      (`KismetSystemLibrary.PrintString` "接続失敗！"))))

(fn `UserConstructionScript`)