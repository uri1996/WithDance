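; Debug actor that calibrates a VR player's body measurements from keyboard presses and stores them in VR_Debug_GameMode.
; On BeginPlay it caches VR_Debug_Pawn, the game mode, and a text block from the Test_UIBP actor's widget.
; M records headset height; V, H and D show Japanese pose prompts (hands up, sideways, down), wait three seconds, then save both grips' raw world Z or Y coordinates as arm lengths.
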(event `self.ReceiveBeginPlay`
  (bind _asvr_debug_pawn (cast `/Game/KubotaBranch/Debug/VR_Debug_Pawn` (`GameplayStatics.GetPlayerPawn` 0)))
  (set `self.PlayerPawn` _asvr_debug_pawn)
  (bind _asvr_debug_game_mode (cast `/Game/KubotaBranch/Debug/VR_Debug_GameMode` (`GameplayStatics.GetGameMode`)))
  (set `self.GameMode` _asvr_debug_game_mode)
  (bind _outactors (`GameplayStatics.GetAllActorsOfClass` "/Game/KubotaBranch/Actor/Test_UIBP.Test_UIBP_C"))
  (bind _astest_ui (cast `/Game/KubotaBranch/Actor/TestUI` (`WidgetComponent.GetWidget` (`/Game/KubotaBranch/Actor/Test_UIBP.Widget` (`|GetArrayItem` _outactors)))))
  (set `self.UIText` (`/Game/KubotaBranch/Actor/TestUI.TextBlock0` _astest_ui)))

(event `Key|M`
  (params (Key :type "Key Structure"))
  (bind (_returnvalue_x _returnvalue_y _returnvalue_z) (`KismetMathLibrary.BreakVector` (`SceneComponent.K2_GetComponentLocation` (`/Game/KubotaBranch/Debug/VR_Debug_Pawn.HeadMountedDisplayMesh` (`self.PlayerPawn`)))))
  (:`Pressed`
    (bind _output_get (set `/Game/KubotaBranch/Debug/VR_Debug_GameMode.HeadHight` _returnvalue_z (`self.GameMode`)))
    (`KismetSystemLibrary.PrintString` (`KismetStringLibrary.Conv_DoubleToString` _output_get))))

(event `Key|V`
  (params (Key :type "Key Structure"))
  (bind _gamemode (`self.GameMode`))
  (bind _uitext (`self.UIText`))
  (bind _playerpawn (`self.PlayerPawn`))
  (bind (_returnvalue_x _returnvalue_y _returnvalue_z) (`KismetMathLibrary.BreakVector` (`SceneComponent.K2_GetComponentLocation` (`/Game/KubotaBranch/Debug/VR_Debug_Pawn.MotionControllerLeftGrip` _playerpawn))))
  (bind (_returnvalue_x_2 _returnvalue_y_2 _returnvalue_z_2) (`KismetMathLibrary.BreakVector` (`SceneComponent.K2_GetComponentLocation` (`/Game/KubotaBranch/Debug/VR_Debug_Pawn.MotionControllerRightGrip` _playerpawn))))
  (:`Pressed`
    (`TextBlock.SetText` (`self.UIText`) "手を上に上げてください")
    (`KismetSystemLibrary.PrintString` "3秒後読み取り")
    (`KismetSystemLibrary.Delay` 3.0)
    (bind _output_get (set `/Game/KubotaBranch/Debug/VR_Debug_GameMode.LArmLength_V` _returnvalue_z _gamemode))
    (`KismetSystemLibrary.PrintString` (`KismetStringLibrary.Conv_DoubleToString` _output_get))
    (bind _output_get_2 (set `/Game/KubotaBranch/Debug/VR_Debug_GameMode.RArmLength_V` _returnvalue_z_2 _gamemode))
    (`KismetSystemLibrary.PrintString` (`KismetStringLibrary.Conv_DoubleToString` _output_get_2))
    (`TextBlock.SetText` _uitext "成功")
    (`KismetSystemLibrary.Delay` 1.0)
    (`TextBlock.SetText` _uitext "")))

(event `Key|H`
  (params (Key :type "Key Structure"))
  (bind _playerpawn (`self.PlayerPawn`))
  (bind _gamemode (`self.GameMode`))
  (bind _uitext (`self.UIText`))
  (bind (_returnvalue_x _returnvalue_y) (`KismetMathLibrary.BreakVector` (`SceneComponent.K2_GetComponentLocation` (`/Game/KubotaBranch/Debug/VR_Debug_Pawn.MotionControllerLeftGrip` _playerpawn))))
  (bind (_returnvalue_x_2 _returnvalue_y_2) (`KismetMathLibrary.BreakVector` (`SceneComponent.K2_GetComponentLocation` (`/Game/KubotaBranch/Debug/VR_Debug_Pawn.MotionControllerRightGrip` _playerpawn))))
  (:`Pressed`
    (`TextBlock.SetText` (`self.UIText`) "手を横に広げてください")
    (`KismetSystemLibrary.PrintString` "3秒後読み取り")
    (`KismetSystemLibrary.Delay` 3.0)
    (bind _output_get (set `/Game/KubotaBranch/Debug/VR_Debug_GameMode.LArmLength_H` _returnvalue_y _gamemode))
    (`KismetSystemLibrary.PrintString` (`KismetStringLibrary.Conv_DoubleToString` _output_get))
    (bind _output_get_2 (set `/Game/KubotaBranch/Debug/VR_Debug_GameMode.RArmLength_H` _returnvalue_y_2 _gamemode))
    (`KismetSystemLibrary.PrintString` (`KismetStringLibrary.Conv_DoubleToString` _output_get_2))
    (`TextBlock.SetText` _uitext "成功")
    (`KismetSystemLibrary.Delay` 1.0)
    (`TextBlock.SetText` _uitext "")))

(event `Key|D`
  (params (Key :type "Key Structure"))
  (bind _playerpawn (`self.PlayerPawn`))
  (bind _uitext (`self.UIText`))
  (bind _gamemode (`self.GameMode`))
  (bind (_returnvalue_x _returnvalue_y _returnvalue_z) (`KismetMathLibrary.BreakVector` (`SceneComponent.K2_GetComponentLocation` (`/Game/KubotaBranch/Debug/VR_Debug_Pawn.MotionControllerLeftGrip` _playerpawn))))
  (bind (_returnvalue_x_2 _returnvalue_y_2 _returnvalue_z_2) (`KismetMathLibrary.BreakVector` (`SceneComponent.K2_GetComponentLocation` (`/Game/KubotaBranch/Debug/VR_Debug_Pawn.MotionControllerRightGrip` _playerpawn))))
  (:`Pressed`
    (`TextBlock.SetText` (`self.UIText`) "手を下に下げてください")
    (`KismetSystemLibrary.PrintString` "3秒後読み取り")
    (`KismetSystemLibrary.Delay` 3.0)
    (bind _output_get (set `/Game/KubotaBranch/Debug/VR_Debug_GameMode.LArmLength_D` _returnvalue_z _gamemode))
    (`KismetSystemLibrary.PrintString` (`KismetStringLibrary.Conv_DoubleToString` _output_get))
    (bind _output_get_2 (set `/Game/KubotaBranch/Debug/VR_Debug_GameMode.RArmLength_D` _returnvalue_z_2 _gamemode))
    (`KismetSystemLibrary.PrintString` (`KismetStringLibrary.Conv_DoubleToString` _output_get_2))
    (`TextBlock.SetText` _uitext "成功")
    (`KismetSystemLibrary.Delay` 1.0)
    (`TextBlock.SetText` _uitext "")))

(fn `UserConstructionScript`)