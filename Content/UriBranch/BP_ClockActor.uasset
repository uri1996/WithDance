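; Rhythm clock actor that plays test background music on a Quartz clock and triggers note generation in time with it.
; StartAudio or the O key creates the clock and queues the sound quantized to the bar.
; Once queued, it starts the clock and subscribes to bar events.
; Every fifth bar, it randomly calls left- or right-hand generation on the GenerateNote actor found at BeginPlay.
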(event `self.ReceiveBeginPlay`
  (bind _outactors (`GameplayStatics.GetAllActorsOfClass` "/Game/KubotaBranch/Actor/GenerateNote.GenerateNote_C"))
  (bind _asgenerate_note (cast `/Game/KubotaBranch/Actor/GenerateNote` (`|GetArrayItem` _outactors)))
  (set `self.GenerateNote` _asgenerate_note))

(event `StartAudio`
  (bind _returnvalue (`QuartzSubsystem.CreateNewClock` (subsystem `QuartzSubsystem`) "NewClock" (make `QuartzClockSettings` (make `QuartzTimeSignature` 4)) false true :!label _label))
  (bind _clockhandle (`QuartzClockHandle.SetBeatsPerMinute` :`self` _returnvalue :`BeatsPerMinute` 90.0))
  (set `self.NewClock` _clockhandle)
  (bind _returnvalue_2 (`GameplayStatics.CreateSound2D` "/Game/UriBranch/TestBGM.TestBGM" 1.0 1.0 0.0 null))
  (`AudioComponent.PlayQuantized` _returnvalue_2 (`self.NewClock`) (make `QuartzQuantizationBoundary` "Bar" 1.0 "TransportRelative") (delegate `Cued`) 0.0 0.0 1.0 "Linear"))

(event `Key|O`
  (params (Key :type "Key Structure"))
  (:`Pressed`
    (goto _label)))

(event `Quantized`
  (params (ClockName :type Name) (QuantizationType :type "EQuartzCommandQuantization Enum" :default "Bar") (NumBars :type Integer) (Beat :type Integer) (BeatFraction :type "Float (single-precision)"))
  (bind _generatenote (`self.GenerateNote`))
  (`KismetSystemLibrary.PrintString` (`KismetStringLibrary.Conv_IntToString` NumBars))
  (if (== (mod NumBars 5) 0)
    (if (== (`KismetMathLibrary.RandomInteger` 2) 0)
      (`/Game/KubotaBranch/Actor/GenerateNote.GenerateNote_handL` _generatenote)
      (else
        (`/Game/KubotaBranch/Actor/GenerateNote.GenerateNote_handR` _generatenote)))))

(event `Cued`
  (params (EventType :type "EQuartzCommandDelegateSubType Enum" :default "CommandOnFailedToQueue") (Name :type Name))
  (switch `EQuartzCommandDelegateSubType` EventType
    (:`CommandOnQueued`
      (bind _clockhandle (`QuartzClockHandle.StartClock` (`self.NewClock`)))
      (`QuartzClockHandle.SubscribeToQuantizationEvent` _clockhandle "Bar" (delegate `Quantized`)))))

(fn `UserConstructionScript`)