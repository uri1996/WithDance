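; BP_FileReader is a test-style reader that pulls text from the Test DataTable and prints it when play begins.
; BeginPlay collects the Words field of every found row into WordArray.
; It joins that array into one string, re-parses it with ParseIntoArray (both separator and delimiter show as empty), and prints each resulting element.
; Tick, overlap and the construction script do nothing.
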(event `self.ReceiveBeginPlay`
  (bind _output_get (set `self.DataTable` "/Game/UriBranch/test.test"))
  (bind _outrownames (`DataTableFunctionLibrary.GetDataTableRowNames` _output_get))
  (for _array_element _outrownames
    (bind _returnvalue (`|GetDataTableRow` (`self.DataTable`) _array_element)
      (:`then`
        (`KismetArrayLibrary.Array_Add` (`self.WordArray`) (`.Words_3_B8FD6D104DB67B2134D8E3A884675154` (break `/Game/UriBranch/TestStruct` _returnvalue))))))
  (bind _output_get_2 (set `self.NewWords` (`KismetStringLibrary.ParseIntoArray` (`KismetStringLibrary.JoinStringArray` (`self.WordArray`)))))
  (for _array_element_2 _output_get_2
    (`KismetSystemLibrary.PrintString` _array_element_2)))

(fn `UserConstructionScript`)