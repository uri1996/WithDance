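; Sound manager actor that creates and controls 2D audio for BGM, sound effects and dance music.
; On BeginPlay it sets a base sound mix and applies each sound type's volume saved in DataManager, or zero when that type's state is off.
; Volume changes override per-category sound classes on that mix and push it.
; Dance music is created from the first entry of an addable song list.
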(event `self.ReceiveBeginPlay`
  (`GameplayStatics.SetBaseSoundMix` "/Game/WuBranch/Sound/SampleSoundMix.SampleSoundMix")
  ;[1 1 1] Data Managerの取得とセット
  (bind _returnvalue (`GameplayStatics.GetActorOfClass` "/Game/WuBranch/Blueprint/DataManager.DataManager_C"))
  (bind _output_get (set `self.saveGameRef` _returnvalue))
  ;[1 1 1] 音量の初期化
  (bind _enumvalue (foreach `/Game/WuBranch/Blueprint/SoundType` false)
    (:`LoopBody`
      (bind _state (`/Game/WuBranch/Blueprint/DataManager.GetState` _output_get _enumvalue))
      (if _state
        (bind _volume (`/Game/WuBranch/Blueprint/DataManager.GetVolume` _output_get _enumvalue))
        (`self.SetInitVolume` _enumvalue _volume)
        (else
          (`self.SetInitVolume` _enumvalue))))))

(fn `AddDanceMusic`
  (params (song :type "SoundCue Object Reference"))
  (`KismetArrayLibrary.Array_Add` (`self.songs`) song))

(fn `ChangeBGMVolume`
  (params (volumn :type "Float (double-precision)"))
  (`GameplayStatics.SetSoundMixClassOverride` "/Game/WuBranch/Sound/SampleSoundMix.SampleSoundMix" "/Game/WuBranch/Sound/BGM/BGMSound.BGMSound" volumn 1.0 0.0)
  (`GameplayStatics.PushSoundMixModifier` "/Game/WuBranch/Sound/SampleSoundMix.SampleSoundMix"))

(fn `ChangeDanceMusicVolume`
  (params (volumn :type "Float (double-precision)"))
  (`GameplayStatics.SetSoundMixClassOverride` "/Game/WuBranch/Sound/SampleSoundMix.SampleSoundMix" "/Game/WuBranch/Sound/Music/DanceMusic.DanceMusic" volumn 1.0 0.0)
  (`GameplayStatics.PushSoundMixModifier` "/Game/WuBranch/Sound/SampleSoundMix.SampleSoundMix"))

(fn `ChangeEffectVolume`
  (params (volumn :type "Float (double-precision)"))
  (`GameplayStatics.SetSoundMixClassOverride` "/Game/WuBranch/Sound/SampleSoundMix.SampleSoundMix" "/Game/WuBranch/Sound/SE/EffectSound.EffectSound" volumn 1.0 0.0)
  (`GameplayStatics.PushSoundMixModifier` "/Game/WuBranch/Sound/SampleSoundMix.SampleSoundMix"))

(fn `ContinuePlayBGM`
  (`AudioComponent.SetPaused` (`self.BGMAudio`) false))

(fn `ContinuePlayDanceMusic`
  (`AudioComponent.SetPaused` (`self.DanceMusicAudio`) false))

(fn `CreateBGM`
  (params (Sound :type "SoundBase Object Reference"))
  (bind _returnvalue (`GameplayStatics.CreateSound2D` Sound 1.0 1.0 0.0 null))
  (set `self.BGMAudio` _returnvalue))

(fn `CreateDanceMusic`
  (bind _songs (`self.songs`))
  (if (`KismetArrayLibrary.Array_IsNotEmpty` _songs)
    (bind _returnvalue (`GameplayStatics.CreateSound2D` (`|GetArrayItem` _songs) 1.0 1.0 0.0 null))
    (set `self.DanceMusicAudio` _returnvalue)))

(fn `CreateSE`
  (params (Sound :type "SoundBase Object Reference"))
  (bind _returnvalue (`GameplayStatics.CreateSound2D` Sound 1.0 1.0 0.0 null))
  (set `self.SEAudio` _returnvalue))

(fn `GetSelectedDanceMusic`
  (returns (song :type "SoundCue Object Reference"))
  (return (`self.selectedSong`)))

(fn `PauseBGM`
  (`AudioComponent.SetPaused` (`self.BGMAudio`) true))

(fn `PauseDanceMusic`
  (`AudioComponent.SetPaused` (`self.DanceMusicAudio`) true))

(fn `PlayBGM`
  (`AudioComponent.Play` (`self.BGMAudio`) 0.0))

(fn `PlayDanceMusic`
  (`AudioComponent.Play` (`self.DanceMusicAudio`) 0.0))

(fn `PlaySE`
  (`AudioComponent.Play` (`self.SEAudio`) 0.0))

(fn `SetInitVolume`
  (params (type :type "/Game/WuBranch/Blueprint/SoundType Enum" :default "NewEnumerator0") (volume :type "Float (double-precision)"))
  (switch `/Game/WuBranch/Blueprint/SoundType` type
    (:`NewEnumerator0`
      (`self.ChangeBGMVolume` volume))
    (:`NewEnumerator1`
      (`self.ChangeEffectVolume` volume))
    (:`NewEnumerator2`
      (`self.ChangeDanceMusicVolume` volume))))

(fn `StopDanceMusic`
  (`AudioComponent.Stop` (`self.DanceMusicAudio`)))

(fn `UserConstructionScript`)