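; DataManager is an actor that persists per-type sound settings, enable state and volume, in a MySaveGame save slot.
; Its construction script caches a save reference, loading the existing slot or creating a new save object if none exists.
; Getters and setters index the SoundsEnable and SoundsVolume arrays by the type converted to an integer, and each setter immediately writes the slot back to disk.
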(fn `ChangeState`
  (params (type :type "/Game/WuBranch/Blueprint/SoundType Enum" :default "NewEnumerator0") (state :type Boolean))
  (`KismetArrayLibrary.Array_Set` (`/Game/WuBranch/Blueprint/MySaveGame.SoundsEnable` (`self.saveRef`)) (`KismetMathLibrary.Conv_ByteToInt` type) state)
  (`self.SaveFile`))

(fn `ChangeVolume`
  (params (type :type "/Game/WuBranch/Blueprint/SoundType Enum" :default "NewEnumerator0") (volume :type "Float (double-precision)"))
  (`KismetArrayLibrary.Array_Set` (`/Game/WuBranch/Blueprint/MySaveGame.SoundsVolume` (`self.saveRef`)) (`KismetMathLibrary.Conv_ByteToInt` type) volume)
  (`self.SaveFile`))

(fn `GetSaveGameRef`
  (returns (saveGameRef :type "/Game/WuBranch/Blueprint/MySaveGame Object Reference"))
  (bind _returnvalue (`GameplayStatics.DoesSaveGameExist` "MySaveGame"))
  (if _returnvalue
    (bind _returnvalue_2 (`GameplayStatics.LoadGameFromSlot` "MySaveGame"))
    (bind _asmy_save_game (cast `/Game/WuBranch/Blueprint/MySaveGame` _returnvalue_2))
    (return _asmy_save_game)
    (else
      (bind _returnvalue_3 (`GameplayStatics.CreateSaveGameObject` "/Game/WuBranch/Blueprint/MySaveGame.MySaveGame_C"))
      (return _returnvalue_3))))

(fn `GetState`
  (params (type :type "/Game/WuBranch/Blueprint/SoundType Enum" :default "NewEnumerator0"))
  (returns (state :type Boolean))
  (return (`|GetArrayItem` (`/Game/WuBranch/Blueprint/MySaveGame.SoundsEnable` (`self.saveRef`)) (`KismetMathLibrary.Conv_ByteToInt` type))))

(fn `GetVolume`
  (params (type :type "/Game/WuBranch/Blueprint/SoundType Enum" :default "NewEnumerator0"))
  (returns (volume :type "Float (double-precision)"))
  (return (`|GetArrayItem` (`/Game/WuBranch/Blueprint/MySaveGame.SoundsVolume` (`self.saveRef`)) (`KismetMathLibrary.Conv_ByteToInt` type))))

(fn `SaveFile`
  (`GameplayStatics.SaveGameToSlot` (`self.saveRef`) "MySaveGame"))

(fn `UserConstructionScript`
  (bind _savegameref (`self.GetSaveGameRef`))
  (set `self.saveRef` _savegameref))