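; PausePanel is an actor with a Widget component that lets the player click a pause panel using left and right trigger inputs.
; On BeginPlay it enables input, caches the pawn's WidgetInteractionComponents (pointer index 0 as left, any other as right) and adds the Trigger_Map mapping context.
; Each trigger press and release simulates a left mouse button on its interaction component.
; Widget clicks and setup only print debug messages; no pause logic is present.
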(event `self.ReceiveBeginPlay`
  (`self.EnableInput` (`GameplayStatics.GetPlayerController` 0))
  (`self.SetWidgetInteractionRef`)
  (`EnhancedInputSubsystemInterface.AddMappingContext` (pcsubsystem `EnhancedInputLocalPlayerSubsystem` (`GameplayStatics.GetPlayerController` 0)) "/Game/WuBranch/Input/Trigger_Map.Trigger_Map" 2 (struct))
  (`KismetSystemLibrary.PrintString` "set trigger map complete" true true (struct :`G` 0.66 :`B` 1.0 :`A` 1.0) 2000.0))

(event `self.Widget.OnClicked`
  (params (TouchedComponent :type "PrimitiveComponent Object Reference") (ButtonPressed :type "Key Structure"))
  (`KismetSystemLibrary.PrintString` (`KismetStringLibrary.Concat_StrStr` (`KismetSystemLibrary.GetDisplayName` TouchedComponent) " Click!") true true (struct :`G` 0.66 :`B` 1.0 :`A` 1.0) 2000.0))

(event `EnhancedInput|/Game/WuBranch/Input/Action/Trigger_Left`
  (params (ActionValue :type Boolean) (ElapsedSeconds :type "Float (double-precision)") (TriggeredSeconds :type "Float (double-precision)") (InputAction :type "InputAction Object Reference" :default "/Game/WuBranch/Input/Action/Trigger_Left.Trigger_Left"))
  (bind _widgetinteractionleft (`self.WidgetInteractionLeft`))
  ;[1 1 1] パースパネルを開けるために
  (:`Started`
    (`WidgetInteractionComponent.PressPointerKey` _widgetinteractionleft "LeftMouseButton"))
  (:`Completed`
    (`WidgetInteractionComponent.ReleasePointerKey` _widgetinteractionleft "LeftMouseButton")))

(event `EnhancedInput|/Game/WuBranch/Input/Action/Trigger_Right`
  (params (ActionValue :type Boolean) (ElapsedSeconds :type "Float (double-precision)") (TriggeredSeconds :type "Float (double-precision)") (InputAction :type "InputAction Object Reference" :default "/Game/WuBranch/Input/Action/Trigger_Right.Trigger_Right"))
  (bind _widgetinteractionright (`self.WidgetInteractionRight`))
  ;[1 1 1] パースパネルを開けるために
  (:`Started`
    (`WidgetInteractionComponent.PressPointerKey` _widgetinteractionright "LeftMouseButton"))
  (:`Completed`
    (`WidgetInteractionComponent.ReleasePointerKey` _widgetinteractionright "LeftMouseButton")))

(fn `SetWidgetInteractionRef`
  (bind _returnvalue (`self.K2_GetComponentsByClass` (`GameplayStatics.GetPlayerPawn` 0) "/Script/UMG.WidgetInteractionComponent"))
  (if (> (`KismetArrayLibrary.Array_Length` _returnvalue) 0)
    (for _array_element _returnvalue
      (if (== (`WidgetInteractionComponent.PointerIndex` _array_element) 0)
        (set `self.WidgetInteractionLeft` _array_element)
        (else
          (set `self.WidgetInteractionRight` _array_element))))
    (else
      (`KismetSystemLibrary.PrintString` "Warning: No WidgetInteractionComponent was found. Menu interaction will FAIL"))))

(fn `UserConstructionScript`)