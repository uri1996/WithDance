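; Game mode for the title screen that registers the player's VR widget interaction components for menu use.
; On BeginPlay it caches the Project_GameInstance, then scans the player pawn for WidgetInteractionComponents.
; Pointer index 0 is stored on the GameInstance as the left hand and any other index as the right.
; It prints a warning if none are found, since menu interaction would fail.
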(event `self.ReceiveBeginPlay`
  (bind _asproject_game_instance (cast `/Game/Main/Blueprints/Project_GameInstance` (`GameplayStatics.GetGameInstance`)))
  (set `self.gameInstance` _asproject_game_instance)
  (`self.SetWidgetInteractionRef`))

(fn `SetWidgetInteractionRef`
  (bind _gameinstance (`self.gameInstance`))
  (bind _returnvalue (`self.K2_GetComponentsByClass` (`GameplayStatics.GetPlayerPawn` 0) "/Script/UMG.WidgetInteractionComponent"))
  (if (> (`KismetArrayLibrary.Array_Length` _returnvalue) 0)
    (for _array_element _returnvalue
      (if (== (`WidgetInteractionComponent.PointerIndex` _array_element) 0)
        (set `/Game/Main/Blueprints/Project_GameInstance.VRLeftHand` _array_element _gameinstance)
        (else
          (set `/Game/Main/Blueprints/Project_GameInstance.VRRightHand` _array_element _gameinstance))))
    (else
      (`KismetSystemLibrary.PrintString` "Warning: No WidgetInteractionComponent was found. Menu interaction will FAIL" true true (struct :`R` 1.0 :`A` 1.0) 20000.0))))

(fn `UserConstructionScript`)