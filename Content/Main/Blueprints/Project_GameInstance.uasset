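; Project game instance that holds score, combo and background music state across the game.
; PlayBGM spawns the given sound as a 2D sound and stores the resulting component in BGM.
; AddScore adds a passed value to Score, while AddCombo increments and ResetCombo clears the combo counter.
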(event `PlayBGM`
  (params (Sound :type "SoundBase Object Reference"))
  (bind _returnvalue (`GameplayStatics.SpawnSound2D` Sound 1.0 1.0 0.0 null true))
  (set `self.BGM` _returnvalue))

(event `/Game/KubotaBranch/Actor/BPI_Interface.AddScore`
  (params (Score :type "Float (double-precision)"))
  (set `self.Score` (+ Score (`self.Score`))))

(event `/Game/KubotaBranch/Actor/BPI_Interface.AddCombo`
  (`/Engine/EditorBlueprintResources/StandardMacros.IncrementInt` (`self.Combo`)))

(event `/Game/KubotaBranch/Actor/BPI_Interface.ResetCombo`
  (set `self.Combo` 0))